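; BP_MyCheatManager is, by its name, a cheat manager, providing a MySpawn function that spawns a requested number of BP_Tree actors.
; MySpawn loops over the amount, spawning each tree at a transform supplied by the RandomPosition helper.
; RandomPosition picks random integer coordinates within a square area centered on the world origin and a narrow height band, setting location only.
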(fn MySpawn
  (params (amount :type Integer))
  (for _index (range 1 amount)
    (Game|SpawnActorfromClass "/Game/BP_Tree.BP_Tree_C" (CallFunction|RandomPosition) "Undefined" "MultiplyWithRoot" 0 0)))

(fn RandomPosition
  (return (Math|Transform|MakeTransform (Math|Vector|MakeVector (Math|Conversions|ToFloat(Integer) (Math|Random|RandomIntegerinRange -2500 2500)) (Math|Conversions|ToFloat(Integer) (Math|Random|RandomIntegerinRange -2500 2500)) (Math|Conversions|ToFloat(Integer) (Math|Random|RandomIntegerinRange 90 190))))))