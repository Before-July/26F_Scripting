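; BP_FloatingActor is an actor that continuously spins and bobs up and down.
; Each Tick adds a local pitch rotation from RotateSpeed, set on BeginPlay, and offsets world Z by a scaled sine of game time.
; Neither motion scales by delta time, so both depend on frame rate.
; Height is set on BeginPlay but does not affect movement.
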(event EventBeginPlay
  (Utilities|FlowControl|Sequence
    (:then_0
      (Variables|Default|Setheight 2e+02))
    (:then_1
      (Variables|Default|Setrotate_speed 5.0))))

(event Collision|EventActorBeginOverlap
  (params (OtherActor :type Actor%20Object%20Reference)))

(event EventTick
  (params (DeltaSeconds :type Float%20%28single-precision%29))
  (bind _returnvalue (Transformation|GetActorLocation))
  (Utilities|FlowControl|Sequence
    (:then_0
      (Transformation|AddActorLocalRotation (Math|Rotator|MakeRotator 0.0 (Variables|Default|Getrotate_speed) 0.0) false false))
    (:then_1
      (Transformation|SetActorLocation (Math|Vector|MakeVector (.x _returnvalue) (.y _returnvalue) (+ (.z _returnvalue) (* (Math|Trig|Sin(Radians) (Utilities|Time|GetTimeSeconds)) 2.0))) false false))))

(fn ConstructionScript)