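; BP_Interactable is an interactable actor whose response to interaction is driven by its DataAsset.
; OnIteract logs the actor's name, destroys it if the asset's Destory flag is set, spawns items, then returns the DataAsset.
; If ItemToSpawn is valid, both of its Blueprint types spawn at the same offset above the actor.
; ParticleEffect is called but does nothing, as its Niagara burst node is disconnected.
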(event EventBeginPlay)

(event Collision|EventActorBeginOverlap
  (params (OtherActor :type Actor%20Object%20Reference)))

(event EventTick
  (params (DeltaSeconds :type Float%20%28single-precision%29)))

(fn ConstructionScript)

(fn Interact
  (Development|PrintString (Utilities|String|Append "interacting " (Utilities|GetDisplayName self))))

(fn Destroy
  (if (Variables|/Game/A1/CollectableItem/PDA_Item.PDA_Item_C|Getdestory (Variables|Default|GetDataAsset))
    (Actor|DestroyActor)))

(fn Spawn
  (bind _returnvalue (Transformation|GetActorTransform))
  (bind _returnvalue_2 (+ (.location _returnvalue) "50.000000,50.000000,300.000000"))
  (bind _returnvalue_3 (Math|Transform|MakeTransform _returnvalue_2 (.rotation _returnvalue) (.scale _returnvalue)))
  (bind _itemtospawn (Variables|/Game/A1/CollectableItem/PDA_Item.PDA_Item_C|GetitemToSpawn (Variables|Default|GetDataAsset))
    (:then
      (Utilities|FlowControl|Sequence
        (:then_0
          (Game|SpawnActorfromClass (Variables|/Game/A1/CollectableItem/PDA_Item.PDA_Item_C|GetBlueprintType _itemtospawn) _returnvalue_3 "Undefined" "MultiplyWithRoot" 0 0))
        (:then_1
          (Game|SpawnActorfromClass (Variables|/Game/A1/CollectableItem/PDA_Item.PDA_Item_C|GetBlueprintType1 _itemtospawn) _returnvalue_3 "Undefined" "MultiplyWithRoot" 0 0))))
    (:else)))

(fn ParticleEffect)

(fn OnIteract
  (CallFunction|Interact)
  (CallFunction|ParticleEffect)
  (CallFunction|Destroy)
  (CallFunction|Spawn)
  (return (Variables|Default|GetDataAsset)))